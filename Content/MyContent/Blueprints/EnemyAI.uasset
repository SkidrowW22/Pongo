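; EnemyAI is an actor that drives an opponent Cube, apparently a paddle, to follow the Pball along the X axis.
; BeginPlay sets the tick interval, and each Tick looks up the ball and reads its Sphere's relative location.
; Move uses MoveComponentTo over MTime toward that clamped X, feeding the Cube's world Y, Z and rotation into the relative target.
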(event `self.ReceiveBeginPlay`
  (`self.SetActorTickInterval` (`self.TickInterval`)))

(event `self.ReceiveTick`
  (params (DeltaSeconds :type "Float (single-precision)"))
  (bind _returnvalue (`GameplayStatics.GetActorOfClass` "/Game/MyContent/Blueprints/Pball.Pball_C"))
  (`/Engine/EditorBlueprintResources/StandardMacros.IsValid` _returnvalue
    (:`Is Valid`
      (set `self.BallLoc` (`SceneComponent.RelativeLocation` (`/Game/MyContent/Blueprints/Pball.Sphere` _returnvalue)))
      (`self.Move`))))

(event `Move`
  (bind _cube (`self.Cube`))
  (bind _ballloc_x (`KismetMathLibrary.BreakVector` (`self.BallLoc`)))
  (bind _returnvalue (`SceneComponent.K2_GetComponentToWorld` _cube))
  (`KismetSystemLibrary.MoveComponentTo` _cube (`KismetMathLibrary.MakeVector` (`KismetMathLibrary.FClamp` _ballloc_x -410.0 670.0) (.y (.location _returnvalue)) (.z (.location _returnvalue))) (.rotation _returnvalue) false false (`self.MTime`)))

(fn `UserConstructionScript`)