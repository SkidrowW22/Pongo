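; Pong ball that launches with a diagonal physics impulse and handles scoring when it hits a side trigger.
; A looping MultiGate on Tick cycles through left-trigger check, right-trigger check and velocity correction, resetting on overlap.
; Velocity correction holds Ballspeed and snaps travel to the nearest diagonal.
; Scoring destroys the ball, updates PongPawn, calls Ball_Spawner for another, and opens NewMap once a side reaches two.
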(event `self.ReceiveBeginPlay`
  (`PrimitiveComponent.AddImpulse` (`self.Sphere`) (-30000.0 30000.0 0.0) "None" false))

(event `VelocityandAngle`
  (bind _returnvalue (`KismetMathLibrary.MakeRotator` 0.0 0.0 45.0))
  (bind _ballspeed (`self.Ballspeed`))
  ;[1 1 1] Velocity and speed control
  (bind _returnvalue_2 (`PrimitiveComponent.GetPhysicsLinearVelocity` (`self.Sphere`) "None"))
  (bind _returnvalue_3 (`KismetMathLibrary.ClampVectorSize` _returnvalue_2 _ballspeed _ballspeed))
  (bind (_returnvalue_roll _returnvalue_pitch _returnvalue_yaw) (`KismetMathLibrary.BreakRotator` (`KismetMathLibrary.MakeRotFromX` (`KismetMathLibrary.GreaterGreater_VectorRotator` _returnvalue_3 _returnvalue))))
  (`PrimitiveComponent.SetPhysicsLinearVelocity` (`self.Sphere`) (* (`KismetMathLibrary.LessLess_VectorRotator` (`KismetMathLibrary.Conv_RotatorToVector` (`KismetMathLibrary.MakeRotator` 0.0 0.0 (`KismetMathLibrary.Conv_IntToDouble` (* (`KismetMathLibrary.Round` (/ _returnvalue_yaw 90.0)) 90)))) _returnvalue) (`KismetMathLibrary.VSize` _returnvalue_3)) false "None"))

(event `self.ReceiveTick`
  (params (DeltaSeconds :type "Float (single-precision)"))
  ;[1 1 1] Scoring system
  (`|MultiGate` false true :!label _label
    (:`Out 0`
      (cast `/Game/MyContent/Blueprints/LeftTrigger` (stale `self.ReceiveActorBeginOverlap` OtherActor))
      (`self.K2_DestroyActor`)
      (bind _aspong_pawn (cast `/Game/MyContent/Blueprints/PongPawn` (`GameplayStatics.GetPlayerPawn` 0)))
      (set `/Game/MyContent/Blueprints/PongPawn.Score_Left` (+ (`/Game/MyContent/Blueprints/PongPawn.Score_Left` _aspong_pawn) 1) _aspong_pawn)
      (bind _outactors (`GameplayStatics.GetAllActorsOfClass` "/Game/MyContent/Blueprints/Ball_Spawner.Ball_Spawner_C"))
      (`/Game/MyContent/Blueprints/Ball_Spawner.SpawnNextB` _outactors)
      (bind _aspong_pawn_2 (cast `/Game/MyContent/Blueprints/PongPawn` (`GameplayStatics.GetPlayerPawn` 0)))
      (if (>= (`/Game/MyContent/Blueprints/PongPawn.Score_Left` _aspong_pawn_2) 2)
        (`KismetSystemLibrary.PrintString` "Left side wins!")
        (`GameplayStatics.OpenLevel` "NewMap")))
    (:`Out 1`
      (cast `/Game/MyContent/Blueprints/RightTrigger` (stale `self.ReceiveActorBeginOverlap` OtherActor))
      (`self.K2_DestroyActor`)
      (bind _aspong_pawn_3 (cast `/Game/MyContent/Blueprints/PongPawn` (`GameplayStatics.GetPlayerPawn` 0)))
      (set `/Game/MyContent/Blueprints/PongPawn.Score_Right` (+ (`/Game/MyContent/Blueprints/PongPawn.Score_Right` _aspong_pawn_3) 1) _aspong_pawn_3)
      (bind _outactors_2 (`GameplayStatics.GetAllActorsOfClass` "/Game/MyContent/Blueprints/Ball_Spawner.Ball_Spawner_C"))
      (`/Game/MyContent/Blueprints/Ball_Spawner.SpawnNextB` _outactors_2)
      (bind _aspong_pawn_4 (cast `/Game/MyContent/Blueprints/PongPawn` (`GameplayStatics.GetPlayerPawn` 0)))
      (if (>= (`/Game/MyContent/Blueprints/PongPawn.Score_Right` _aspong_pawn_4) 2)
        (`KismetSystemLibrary.PrintString` "Right side wins!")
        (`GameplayStatics.OpenLevel` "NewMap")))
    (:`Out 2`
      ;[1 1 1] Velocity and speed control
      (`self.VelocityandAngle`))))

(event `self.ReceiveActorBeginOverlap`
  (params (OtherActor :type "Actor Object Reference"))
  ;[1 1 1] Scoring system
  (goto _label :!via `Reset`))

(fn `UserConstructionScript`)